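; Test actor that connects to a Datasmith DirectLink source at runtime.
; On BeginPlay it spawns a DatasmithRuntimeActor as its anchor, caches the DirectLink proxy and calls DirectLinkUpdate.
; That function stores the available source list, sets the anchor's import options for tessellation and collision, then opens a connection by the SourceIndex variable.
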(event `self.ReceiveBeginPlay`
  (bind _returnvalue (`|SpawnActorFromClass` "/Script/DatasmithRuntime.DatasmithRuntimeActor" (`KismetMathLibrary.MakeTransform` (0.0 0.0 0.0)) "Undefined" "MultiplyWithRoot" null null))
  (set `self.Anchor` _returnvalue)
  (bind _returnvalue_2 (`DatasmithRuntimeLibrary.GetDirectLinkProxy`))
  (set `self.DirectLinkProxy` _returnvalue_2)
  (`self.DirectLinkUpdate`))

(fn `DirectLinkUpdate`
  (bind _anchor (`self.Anchor`))
  (bind _returnvalue (`DirectLinkProxy.GetListOfSources` (`self.DirectLinkProxy`)))
  (set `self.Sources` _returnvalue)
  (set `DatasmithRuntimeActor.ImportOptions` (make `DatasmithRuntimeImportOptions` (make `DatasmithTessellationOptions` 0.05 0.0 5.0) "Unfiltered" "NoCollision") _anchor)
  (`DatasmithRuntimeActor.OpenConnectionWithIndex` _anchor (`self.Source Index`)))

(fn `UserConstructionScript`)